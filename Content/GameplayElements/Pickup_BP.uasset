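; Pong pickup Blueprint that applies a speed, size or ice effect to the paddle that last hit.
; UsePickup switches on PickupType and edits the player's or enemy's paddle struct in Pong_GM, chosen by PlayerLastHit.
; Speed and size variants then call SpeedPickup or SizePickup on that paddle actor, while Ice only sets the Icy flag.
; The graph contains no overlap or spawn logic, only this effect event.
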(event `Use Pickup`
  (bind _aspong_gm (cast `/Game/Pong_GM` (`GameplayStatics.GetGameMode`)))
  (switch `/Game/PickupType_Enum` (`self.PickupType`)
    (:`NewEnumerator0`
      (bind _returnvalue (select `bool` (`/Game/Pong_GM.PlayerLastHit` _aspong_gm) :`false` (`/Game/Pong_GM.EnemyPaddle_Info` _aspong_gm) :`true` (`/Game/Pong_GM.PlayerPaddle_Info` _aspong_gm)))
      (setmembers `/Game/Paddle_Struct` :`StructRef` _returnvalue :`Speed` 1.5)
      (bind _paddle_actor (break `/Game/Paddle_Struct` _returnvalue))
      (`/Game/GameplayElements/PlayerPaddle.SpeedPickup` _paddle_actor :!label _label))
    (:`NewEnumerator1`
      (setmembers `/Game/Paddle_Struct` :`StructRef` _returnvalue :`Speed` 0.5)
      (goto _label))
    (:`NewEnumerator2`
      (setmembers `/Game/Paddle_Struct` :`StructRef` _returnvalue :`Size` 2.0)
      (`/Game/GameplayElements/PlayerPaddle.SizePickup` _paddle_actor :!label _label_2))
    (:`NewEnumerator3`
      (setmembers `/Game/Paddle_Struct` :`StructRef` _returnvalue :`Size` 0.5)
      (goto _label_2))
    (:`NewEnumerator4`
      (setmembers `/Game/Paddle_Struct` :`StructRef` _returnvalue :`Icy` true))))

(fn `UserConstructionScript`)